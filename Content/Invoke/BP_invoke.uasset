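; BP_invoke is an actor with health that attacks any BP_Tower entering its collision sphere.
; On overlap it starts a delay-driven loop that applies AttackDamage at a rate set by AttackSpeed, with no exit condition.
; AnyDamage prints and subtracts incoming damage, destroying the actor at zero health or below.
; SetHealthValue sets current health, and GetHealthPct returns current times max health over 10000 rather than a true ratio.
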(event OnComponentBeginOverlap(CollisionSphere)
  (params (OverlappedComponent :type Primitive%20Component%20Object%20Reference) (OtherActor :type Actor%20Object%20Reference) (OtherComp :type Primitive%20Component%20Object%20Reference) (OtherBodyIndex :type Integer) (bFromSweep :type Boolean) (SweepResult :type Hit%20Result%20Structure%20%28by%20ref%29))
  (if (== (Utilities|GetClass OtherActor) "/Game/Tower/BP_Tower.BP_Tower_C")
    (Game|Damage|ApplyDamage OtherActor (Variables|Default|GetAttackDamage) 0 self :!label _label)
    (Utilities|FlowControl|Delay (/ 1.0 (Variables|Default|GetAttackSpeed)))
    (goto _label)))

(event EventBeginPlay)

(event Collision|EventActorBeginOverlap
  (params (OtherActor :type Actor%20Object%20Reference)))

(event EventTick
  (params (DeltaSeconds :type Float%20%28single-precision%29)))

(event Game|Damage|EventAnyDamage
  (params (Damage :type Float%20%28single-precision%29) (DamageType :type Damage%20Type%20Object%20Reference) (InstigatedBy :type Controller%20Object%20Reference) (DamageCauser :type Actor%20Object%20Reference))
  (Development|PrintString (Utilities|String|ToString(Float) Damage))
  (bind _output_get (Variables|Default|SetCurrentHealth (- (Variables|Default|GetCurrentHealth) Damage)))
  (if (<= _output_get 0)
    (Actor|DestroyActor)))

(event EventSetHealthValue
  (params (health :type Float%20%28double-precision%29))
  (Variables|Default|SetCurrentHealth (Math|Float|Truncate health)))

(fn ConstructionScript)

(fn GetHealthPct
  (return (/ (* (Variables|Default|GetCurrentHealth) (Variables|Default|GetMaxHealth)) 10000)))