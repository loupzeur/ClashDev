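; Tower actor that damages overlapping BP_invoke units and can itself be destroyed.
; FireCollision overlaps add units to SelectedEnemy, which a self-restarting delayed loop works through, hitting one target every second until it is invalid, then removing it.
; Damage taken lowers CurrentHealth; at zero the tower destroys itself and leaves G_Clash's ActiveTowers.
; It registers as owner of its W_Health widget and exposes a health ratio.
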(event OnComponentBeginOverlap(FireCollision)
  (params (OverlappedComponent :type Primitive%20Component%20Object%20Reference) (OtherActor :type Actor%20Object%20Reference) (OtherComp :type Primitive%20Component%20Object%20Reference) (OtherBodyIndex :type Integer) (bFromSweep :type Boolean) (SweepResult :type Hit%20Result%20Structure%20%28by%20ref%29))
  (bind _asbp_invoke (Utilities|Casting|CastToBP_invoke OtherActor))
  (Utilities|Array|AddUnique (Variables|Default|GetSelectedEnemy) _asbp_invoke))

(event Custom|GenerateDamage
  (bind _selectedenemy (Variables|Default|GetSelectedEnemy))
  (bind (_array_element _array_index) (Utilities|Array|ForEachLoopwithBreak _selectedenemy :!label _label)
    (:LoopBody
      (Utilities|IsValid _array_element :!label _label_2
        (:Is%20Valid
          (Game|Damage|ApplyDamage _array_element (Math|Conversions|ToFloat(Integer) (Variables|Default|GetAttackDamage)) 0 self)
          (Utilities|FlowControl|Delay 1.0)
          (goto _label_2))
        (:Is%20Not%20Valid
          (Utilities|Array|RemoveIndex _selectedenemy _array_index)
          (goto _label Break))))
    (:Completed
      (Utilities|FlowControl|Delay 1.0)
      (goto _label))))

(event EventBeginPlay
  (bind _asw_health (Utilities|Casting|CastToW_Health (UserInterface|GetWidget (Variables|Default|GetHealth_0))))
  (Variables|/Game/UI/W_Health.W_Health_C|SetOwnerObject _asw_health self)
  (CallFunction|GenerateDamage))

(event Game|Damage|EventAnyDamage
  (params (Damage :type Float%20%28single-precision%29) (DamageType :type Damage%20Type%20Object%20Reference) (InstigatedBy :type Controller%20Object%20Reference) (DamageCauser :type Actor%20Object%20Reference))
  (Variables|Default|SetCurrentHealth (Math|Float|Truncate (- (Variables|Default|GetCurrentHealth) Damage)))
  (if (<= (- (Variables|Default|GetCurrentHealth) Damage) 0.0)
    (Actor|DestroyActor)
    (bind _asg_clash (Utilities|Casting|CastToG_Clash (Game|GetGameMode)))
    (Utilities|Array|RemoveItem (Variables|/Game/G_Clash.G_Clash_C|GetActiveTowers _asg_clash) self)))

(event EventSetHealthValue
  (params (health :type Float%20%28double-precision%29))
  (Variables|Default|SetCurrentHealth (Math|Float|Truncate health)))

(fn ConstructionScript)

(fn GetHealthPct
  (return (/ (Variables|Default|GetCurrentHealth) (Variables|Default|GetMaxHealth))))